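; FloorLevelBP is a level generator actor that builds a grid of Room actors when play begins.
; It loops over the nested RoomStates rows and spawns a Room per entry, offset from its own location at a fixed grid spacing with its rotation and scale.
; Each entry's boolean flags decide which front, back, left and right walls the new room adds.
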(event EventBeginPlay
  (bind _returnvalue (Transformation|GetActorTransform))
  (bind (_location _rotation _scale) (Math|Transform|BreakTransform _returnvalue))
  (for (_array_element _array_index) (Variables|Default|GetRoomStates)
    (for (_array_element_2 _array_index_2) (Utilities|Struct|BreakRoomsRow _array_element)
      (bind _returnvalue_2 (Game|SpawnActorfromClass "/Game/Blueprints/Room.Room_C" (Math|Transform|MakeTransform (+ (Math|Vector|MakeVector (* _array_index_2 8e+02) (* _array_index 8e+02) 0.0) _location) _rotation _scale) "Undefined" 0 0))
      (Utilities|FlowControl|Sequence
        (:then_0
          (if (.HasFrontWall (Utilities|Struct|BreakRoomState _array_element_2))
            (Default|AddFrontWall _returnvalue_2)))
        (:then_1
          (if (.HasBackWall (Utilities|Struct|BreakRoomState _array_element_2))
            (Default|AddBackWall _returnvalue_2)))
        (:then_2
          (if (.HasLeftWall (Utilities|Struct|BreakRoomState _array_element_2))
            (Default|AddLeftWall _returnvalue_2)))
        (:then_3
          (if (.HasRightWall (Utilities|Struct|BreakRoomState _array_element_2))
            (Default|AddRightWall _returnvalue_2)))))))

(fn ConstructionScript)