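; Room is an actor Blueprint that can spawn walls on its four sides.
; Four functions, one each for front, left, right and back, spawn a Wall actor at the world transform of that side's attach component.
; The event graph and construction script are empty, so the Room does not call these functions itself.
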(event EventBeginPlay)

(event Collision|EventActorBeginOverlap
  (params (OtherActor :type Actor%20Object%20Reference)))

(event EventTick
  (params (DeltaSeconds :type Float%20%28single-precision%29)))

(fn ConstructionScript)

(fn AddFrontWall
  (Game|SpawnActorfromClass "/Game/Blueprints/Wall.Wall_C" (Transformation|GetWorldTransform (Variables|Default|GetfrontWallAttach)) "Undefined" 0 0))

(fn AddLeftWall
  (Game|SpawnActorfromClass "/Game/Blueprints/Wall.Wall_C" (Transformation|GetWorldTransform (Variables|Default|GetleftWallAttach)) "Undefined" 0 0))

(fn AddRightWall
  (Game|SpawnActorfromClass "/Game/Blueprints/Wall.Wall_C" (Transformation|GetWorldTransform (Variables|Default|GetrightWallAttach)) "Undefined" 0 0))

(fn AddBackWall
  (Game|SpawnActorfromClass "/Game/Blueprints/Wall.Wall_C" (Transformation|GetWorldTransform (Variables|Default|GetbackWallAttack)) "Undefined" 0 0))